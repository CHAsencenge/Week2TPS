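; Cannonball projectile actor that explodes once it slows down, rather than on impact; its hit event is empty.
; Every Tick it computes the CannonSphere's speed from its velocity components and compares it to a fixed threshold.
; Below that, it activates RadialForce, spawns explosion particles and sound at the sphere, then destroys itself after a short delay.
; No guard stops the effects re-spawning each slow frame during that delay.
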(event `self.CannonSphere.OnComponentHit`
  (params (HitComponent :type "PrimitiveComponent Object Reference") (OtherActor :type "Actor Object Reference") (OtherComp :type "PrimitiveComponent Object Reference") (NormalImpulse :type "Vector Structure") (Hit :type "HitResult Structure (by ref)")))

(event `self.ReceiveTick`
  (params (DeltaSeconds :type "Float (single-precision)"))
  (bind _returnvalue (`SceneComponent.K2_GetComponentLocation` (`self.CannonSphere`)))
  (if (< (`KismetMathLibrary.Sqrt` (+ (`KismetMathLibrary.Square` (.x (`SceneComponent.GetComponentVelocity` (`self.CannonSphere`)))) (`KismetMathLibrary.Square` (.y (`SceneComponent.GetComponentVelocity` (`self.CannonSphere`)))) (`KismetMathLibrary.Square` (.z (`SceneComponent.GetComponentVelocity` (`self.CannonSphere`)))))) 350.0)
    (`ActorComponent.Activate` (`self.RadialForce`) false)
    (`GameplayStatics.SpawnEmitterAtLocation` "/Game/SciFiWeapLight/FX/Particles/P_Grenade_Explosion_Dark.P_Grenade_Explosion_Dark" _returnvalue)
    (`GameplayStatics.SpawnSoundAtLocation` "/Game/SciFiWeapLight/Sound/GrenadeLauncher/Wavs/GL_Explosion01.GL_Explosion01" _returnvalue (struct) 1.0 1.0 0.0 null null)
    (`KismetSystemLibrary.Delay` 0.1)
    (`self.K2_DestroyActor`)))

(fn `UserConstructionScript`)