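; Wall Blueprint that plays impact effects when specific projectile-like spheres overlap its static mesh.
; On begin overlap it identifies the other component by comparing its object name to hard-coded strings.
; "Sphere1" triggers a stone impact emitter and shotgun impact sound, while "CannonSphere" triggers a grenade explosion emitter and sound.
; Effects spawn at the overlapping component's location, and the wall itself is left unchanged.
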(event `self.StaticMeshComponent.OnComponentBeginOverlap`
  (params (OverlappedComponent :type "PrimitiveComponent Object Reference") (OtherActor :type "Actor Object Reference") (OtherComp :type "PrimitiveComponent Object Reference") (OtherBodyIndex :type Integer) (bFromSweep :type Boolean) (SweepResult :type "HitResult Structure (by ref)"))
  (bind _returnvalue (`SceneComponent.K2_GetComponentLocation` OtherComp))
  (bind _returnvalue_2 (`KismetSystemLibrary.GetObjectName` OtherComp))
  (if (`KismetStringLibrary.EqualEqual_StrStr` _returnvalue_2 "Sphere1")
    (`GameplayStatics.SpawnEmitterAtLocation` "/Game/SciFiWeapLight/FX/Particles/P_Impact_Stone_Large_Dark.P_Impact_Stone_Large_Dark" _returnvalue)
    (`GameplayStatics.SpawnSoundAtLocation` "/Game/SciFiWeapLight/Sound/Shotgun/Wavs/Shotgun_ImpactSurface02.Shotgun_ImpactSurface02" _returnvalue (struct) 1.0 1.0 0.0 null null)
    (elif (`KismetStringLibrary.EqualEqual_StrStr` _returnvalue_2 "CannonSphere")
      (`GameplayStatics.SpawnEmitterAtLocation` "/Game/SciFiWeapLight/FX/Particles/P_Grenade_Explosion_Light.P_Grenade_Explosion_Light" _returnvalue)
      (`GameplayStatics.SpawnSoundAtLocation` "/Game/SciFiWeapLight/Sound/GrenadeLauncher/Wavs/GL_Explosion02.GL_Explosion02" _returnvalue (struct) 1.0 1.0 0.0 null null))))

(fn `UserConstructionScript`
  (`parent.UserConstructionScript`))