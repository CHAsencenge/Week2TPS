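; White grenade launcher weapon Blueprint that fires Cannon actors and feeds an aim point to the shooting HUD.
; Fire spawns a Cannon at the mesh's Muzzle socket along with a small impact particle effect.
; Every Tick, a visibility trace runs from just above the muzzle along the mesh's right vector, passing the hit location to ShootHUD through GetLocation.
; An explosion emitter at the hit point is left unconnected.
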(event `Fire`
  (bind _returnvalue (`SceneComponent.GetSocketTransform` (`self.SkeletalMesh`) "Muzzle" "RTS_World"))
  (`|SpawnActorFromClass` "/Game/BluePrints/Cannon.Cannon_C" _returnvalue "Undefined" "OverrideRootScale" null null)
  (`GameplayStatics.SpawnEmitterAtLocation` "/Game/SciFiWeapLight/FX/Particles/P_Impact_Wood_Small_Dark.P_Impact_Wood_Small_Dark" (.location _returnvalue)))

(event `self.ReceiveTick`
  (params (DeltaSeconds :type "Float (single-precision)"))
  (bind _returnvalue (+ (.location (`SceneComponent.GetSocketTransform` (`self.SkeletalMesh`) "Muzzle" "RTS_World")) (0.0 0.0 6.0)))
  (bind _outhit (`KismetSystemLibrary.LineTraceSingle` _returnvalue (+ _returnvalue (* (`SceneComponent.GetRightVector` (`self.SkeletalMesh`)) 15000.0)) "TraceTypeQuery1"))
  (bind _foundwidgets (`WidgetBlueprintLibrary.GetAllWidgetsOfClass` "/Game/BluePrints/ShootHUD.ShootHUD_C"))
  (`/Game/BluePrints/ShootHUD.GetLocation` _foundwidgets (`.Location` (`GameplayStatics.BreakHitResult` _outhit))))

(fn `UserConstructionScript`)