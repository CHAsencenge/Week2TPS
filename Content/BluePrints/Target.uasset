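; Target is a scoring target actor that awards points based on where it is hit.
; On BeginPlay it creates a PointsHUD widget, adds it to the viewport and keeps it to hold the cumulative score.
; Each Hit measures the hit location's Y/Z distance from a hardcoded world-space center, adding 3, 2 or 1 points for inner, middle or outer zones.
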(event `self.ReceiveHit`
  (params (MyComp :type "PrimitiveComponent Object Reference") (Other :type "Actor Object Reference") (OtherComp :type "PrimitiveComponent Object Reference") (bSelfMoved :type Boolean) (HitLocation :type "Vector Structure") (HitNormal :type "Vector Structure") (NormalImpulse :type "Vector Structure") (Hit :type "HitResult Structure (by ref)"))
  (bind _returnvalue (`KismetMathLibrary.VSize2D` (- (`KismetMathLibrary.MakeVector2D` (.y HitLocation) (.z HitLocation)) (760.0 220.0))))
  (`KismetSystemLibrary.PrintText` "Hit Target" false)
  (if (< _returnvalue 20.0)
    (bind _output_get (set `/Game/BluePrints/PointsHUD.CumPoints` (+ 3 (`/Game/BluePrints/PointsHUD.CumPoints` (stale `self.ReceiveBeginPlay` _returnvalue))) (stale `self.ReceiveBeginPlay` _returnvalue)))
    (`KismetSystemLibrary.PrintText` (`KismetTextLibrary.Conv_IntToText` _output_get) false)
    (elif (< _returnvalue 50.0)
      (bind _output_get_2 (set `/Game/BluePrints/PointsHUD.CumPoints` (+ 2 (`/Game/BluePrints/PointsHUD.CumPoints` (stale `self.ReceiveBeginPlay` _returnvalue))) (stale `self.ReceiveBeginPlay` _returnvalue)))
      (`KismetSystemLibrary.PrintText` (`KismetTextLibrary.Conv_IntToText` _output_get_2) false)
      (else
        (bind _output_get_3 (set `/Game/BluePrints/PointsHUD.CumPoints` (+ 1 (`/Game/BluePrints/PointsHUD.CumPoints` (stale `self.ReceiveBeginPlay` _returnvalue))) (stale `self.ReceiveBeginPlay` _returnvalue)))
        (`KismetSystemLibrary.PrintText` (`KismetTextLibrary.Conv_IntToText` _output_get_3) false)))))

(event `self.ReceiveBeginPlay`
  (bind _returnvalue (`|CreateWidget` "/Game/BluePrints/PointsHUD.PointsHUD_C"))
  (`UserWidget.AddToViewport` _returnvalue 0))

(fn `UserConstructionScript`)